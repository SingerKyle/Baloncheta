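; BP_Instantiator is a construction-time tool that tiles a chosen static mesh into a flat X-by-Y grid.
; The construction script assigns the mesh to an InstancedStaticMesh component, then nested loops add one local-space instance per cell.
; Cell spacing comes from the mesh's bounding box size on each axis, so tiles sit edge to edge.
; The event graph holds only disabled stub events.
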(event EventBeginPlay)

(event Collision|EventActorBeginOverlap
  (params (OtherActor :type Actor%20Object%20Reference)))

(event EventTick
  (params (DeltaSeconds :type Float%20%28single-precision%29)))

(fn ConstructionScript
  (bind _staticmesh (Variables|Default|GetStaticMesh))
  (bind _returnvalue (StaticMesh|GetBoundingBox _staticmesh))
  (bind (_x _y) (Math|Vector|BreakVector (.min _returnvalue)))
  (bind (_x_2 _y_2) (Math|Vector|BreakVector (.max _returnvalue)))
  (Components|StaticMesh|SetStaticMesh (Variables|Default|GetInstancedStaticMesh) (Variables|Default|GetStaticMesh))
  (for _index (range 0 (- (Variables|Default|GetYInstances) 1))
    (LocalVariables|SetYIndex _index)
    (for _index_2 (range 0 (- (Variables|Default|GetXInstances) 1))
      (LocalVariables|SetXIndex _index_2)
      (Components|InstancedStaticMesh|AddInstance (Variables|Default|GetInstancedStaticMesh) (Math|Transform|MakeTransform (Math|Vector|MakeVector (* (- _x_2 _x) (LocalVariables|GetXIndex)) (* (- _y_2 _y) (LocalVariables|GetYIndex)) 0.0)) false))))