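; VR game mode that runs a timed bubble-scoring round, from start through game over to a level reload on restart.
; StartGame and a timer-driven FinishGame toggle the bubble spawner's tick, swap start, scoreboard and game-over actors, and fire MetaSound triggers to shift the music.
; Combo scales points per bubble, while penalties subtract the last amount added.
; Score and combo changes broadcast through dispatchers, and score changes spawn world-space pop-ups.
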(event Custom|StartGame
  (bind _music (Variables|Default|GetMusic))
  (if (Variables|Default|GetIsGameOver?)
    (CallFunction|ResetGame)
    (elif (not (Variables|Default|GetIsGameLive?))
      (bind _returnvalue (Actor|GetActorOfClass "/Game/Baloncheta/Blueprint/BP_BubbleSpawner.BP_BubbleSpawner_C"))
      (Actor|Tick|SetActorTickEnabled _returnvalue true)
      (Utilities|Time|SetTimerbyEvent (delegate Custom|FinishGame) (Variables|Default|GetGameDuration))
      (Variables|Default|SetIsGameLive? true)
      (bind _returnvalue_2 (Actor|GetActorOfClass "/Game/Baloncheta/Blueprint/WBP_GameStartActor.WBP_GameStartActor_C"))
      (Actor|DestroyActor _returnvalue_2)
      (Class|AudioParameterControllerInterface|SetTriggerParameter _music "MainRelease")
      (Class|AudioParameterControllerInterface|SetTriggerParameter _music "PlayAttack"))))

(event Custom|FinishGame
  (bind _music (Variables|Default|GetMusic))
  (bind _returnvalue (Actor|GetActorOfClass "/Game/Baloncheta/Blueprint/BP_BubbleSpawner.BP_BubbleSpawner_C"))
  (Actor|Tick|SetActorTickEnabled _returnvalue)
  (bind _outactors (Actor|GetAllActorsOfClass "/Game/Baloncheta/Blueprint/BP_Bubble.BP_Bubble_C"))
  (for _array_element _outactors
    (Actor|DestroyActor _array_element))
  (Variables|Default|SetIsGameOver? true)
  (bind _returnvalue_2 (Game|SpawnActorfromClass "/Game/Baloncheta/Blueprint/WBP_GameOverActor.WBP_GameOverActor_C" (Math|Transform|MakeTransform "500.000000,-150.000000,320.000000" "0.000000,90.000000,0.000000" "0.500000,0.500000,0.500000") "Undefined" "MultiplyWithRoot" self (Game|Player|GetPlayerPawn 0)))
  (bind _aswbp_game_over (Utilities|Casting|CastToWBP_GameOver (UserInterface|GetWidget (Variables|/Game/Baloncheta/Blueprint/WBP_GameOverActor.WBP_GameOverActor_C|GetWidget _returnvalue_2))))
  (Rendering|Components|TextRender|SetText (Variables|/Game/Baloncheta/Widget/WBP_GameOver.WBP_GameOver_C|GetScore _aswbp_game_over) (Utilities|Text|ToText(Float) (Variables|Default|GetScore) "HalfToEven" false true 1 324 0 0))
  (bind _returnvalue_3 (Actor|GetActorOfClass "/Game/Baloncheta/Blueprint/BP_Scoreboard.BP_Scoreboard_C"))
  (Actor|DestroyActor _returnvalue_3)
  (Class|AudioParameterControllerInterface|SetTriggerParameter _music "PlayRelease")
  (Class|AudioParameterControllerInterface|SetTriggerParameter _music "EndAttack"))

(event EventBeginPlay
  (bind _returnvalue (Audio|SpawnSound2D "/Game/Baloncheta/SFX/Music/MS_Music.MS_Music" 1.0 1.0 0.0 0))
  (Variables|Default|SetMusic _returnvalue))

(fn ConstructionScript)

(fn IncreaseScore
  (params (Location :type Vector))
  (bind _scoreperbubble (Variables|Default|GetScorePerBubble))
  (bind _combo (Variables|Default|GetCombo))
  (bind _returnvalue (* _combo 0.1))
  (bind _returnvalue_2 (* _scoreperbubble _returnvalue))
  (bind _output_get (Variables|Default|SetScore (+ (Variables|Default|GetScore) _returnvalue_2)))
  (bind _output_get_2 (Variables|Default|SetLastScoreAdded _returnvalue_2))
  (Default|CallOnScoreUpdated _output_get _output_get_2)
  (bind _returnvalue_3 (Game|SpawnActorfromClass "/Game/Baloncheta/Blueprint/WBP_ScorePop.WBP_ScorePop_C" (Math|Transform|MakeTransform Location "0.000000,90.000000,0.000000" "0.500000,0.500000,0.500000") "Undefined" "MultiplyWithRoot" 0 0))
  (Default|SetNumber _returnvalue_3 (Math|Float|Truncate (Variables|Default|GetLastScoreAdded))))

(fn IncreaseCombo
  (bind _result (Math|Integer|IncrementInt (Variables|Default|GetCombo))
    (:%20%20
      (Default|CallOnComboUpdated _result))))

(fn LoseCombo
  (bind _output_get (Variables|Default|SetCombo 0))
  (Default|CallOnComboUpdated _output_get))

(fn DecreaseScore
  (params (Location :type Vector))
  (LocalVariables|SetLastScoreLocal (Variables|Default|GetLastScoreAdded))
  (bind _output_get (Variables|Default|SetScore (Math|Float|Max(Float) (- (Variables|Default|GetScore) (Variables|Default|GetLastScoreAdded)) 0.0)))
  (Variables|Default|SetLastScoreAdded 1e+02)
  (Default|CallOnScoreUpdated _output_get (* (LocalVariables|GetLastScoreLocal) -1.0))
  (bind _returnvalue (Game|SpawnActorfromClass "/Game/Baloncheta/Blueprint/WBP_ScorePop.WBP_ScorePop_C" (Math|Transform|MakeTransform Location "0.000000,90.000000,0.000000" "0.500000,0.500000,0.500000") "Undefined" "MultiplyWithRoot" 0 0))
  (Default|SetNumber _returnvalue (* (Math|Float|Truncate (Variables|Default|GetLastScoreAdded)) -1)))

(fn ResetGame
  (Game|OpenLevel(byObjectReference) "/Game/Baloncheta/Map/L_Main.L_Main"))