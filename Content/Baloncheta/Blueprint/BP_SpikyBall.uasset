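; BP_SpikyBall is a VR hazard that penalizes the player when hit by a hand.
; Tick drifts it along world Y at Speed while a per-frame sine offset bobs it on Z, with the wave rate randomized at BeginPlay.
; HandHit calls HitFeedback, which breaks the combo and lowers score through VRGameMode and spawns a bad-pop sound and spiky burst effect, then destroys the actor.
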(event EventHandHit
  (params (Hand :type E_Hand%20Enum :default "NewEnumerator0") (Hit :type Hit%20Result%20Structure))
  (CallFunction|HitFeedback false)
  (Actor|DestroyActor))

(event EventBeginPlay
  (Variables|Default|SetSine%20Speed (Math|Random|RandomFloatinRange 2e+02 4e+02)))

(event EventTick
  (params (DeltaSeconds :type Float%20%28single-precision%29))
  (Transformation|AddActorWorldOffset (Math|Vector|MakeVector 0.0 (* (Variables|Default|GetSpeed) (Utilities|Time|GetWorldDeltaSeconds)) (Math|Trig|Sin(Degrees) (Variables|Default|GetDegrees))))
  (Variables|Default|SetDegrees (Math|Float|%(Float) (+ (Variables|Default|GetDegrees) (* DeltaSeconds (Variables|Default|GetSine%20Speed))) 3.6e+02)))

(fn ConstructionScript)

(fn HitFeedback
  (params (bSuccessfulHit? :type Boolean))
  (bind _returnvalue (Game|GetGameMode))
  (bind _returnvalue_2 (Transformation|GetActorLocation))
  (bind _asvrgame_mode (Utilities|Casting|CastToVRGameMode _returnvalue))
  (Default|LoseCombo _asvrgame_mode)
  (Default|DecreaseScore _asvrgame_mode)
  (Audio|SpawnSoundatLocation "/Game/Baloncheta/SFX/NegativePop/MS_BadPop.MS_BadPop" _returnvalue_2 "0, 0, 0" 1.0 1.0 0.0 0 0)
  (Niagara|SpawnSystematLocation "/Game/Baloncheta/Niagara/NS_BubbleBurst_Spiky.NS_BubbleBurst_Spiky" _returnvalue_2))