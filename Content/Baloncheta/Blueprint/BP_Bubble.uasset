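; BP_Bubble is a bubble target for a VR game, assigned to a particular hand and scored when hit.
; HandHit compares the striking hand to BubbleHand, passes the result to HitFeedback, then destroys the bubble whether or not the hand matched.
; HitFeedback calls VRGameMode to increase combo and score on a match, or to lose the combo on a mismatch.
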(event EventTick
  (params (DeltaSeconds :type Float%20%28single-precision%29)))

(event EventHandHit
  (params (Hand :type E_Hand%20Enum :default "NewEnumerator0"))
  (CallFunction|HitFeedback (Utilities|Enum|Equal(Enum) Hand (Variables|Default|GetBubbleHand)))
  (Actor|DestroyActor))

(fn ConstructionScript)

(fn HitFeedback
  (params (bSuccessfulHit? :type Boolean))
  (bind _returnvalue (Game|GetGameMode))
  (bind _asvrgame_mode (Utilities|Casting|CastToVRGameMode _returnvalue))
  (if bSuccessfulHit?
    (Default|IncreaseCombo _asvrgame_mode)
    (Default|IncreaseScore _asvrgame_mode)
    (else
      (Default|LoseCombo _asvrgame_mode))))