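; Bubble spawner actor that repeatedly fires BP_Bubble actors from its Cylinder component.
; Tick drives a two-state OctoState loop: a DoOnce sets Moving and starts the ShootCooldown timeline, whose finish switches to Shooting.
; Shooting spawns one bubble and resets the DoOnce, restarting the cooldown on the following tick.
; Each bubble gets one of two hand types at random and a limited lifespan.
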(event Custom|Shoot
  (bind _returnvalue (Game|SpawnActorfromClass "/Game/Baloncheta/Blueprint/BP_Bubble.BP_Bubble_C" (Transformation|GetWorldTransform (Variables|Default|GetCylinder)) "AlwaysSpawn" "MultiplyWithRoot" self 0))
  (bind _output_get (Variables|Default|SetBubble _returnvalue))
  (Default|SetBubbleHand _output_get (select (Math|Random|RandomBool) "NewEnumerator1" "NewEnumerator0"))
  (Actor|SetLifeSpan _output_get 6.0))

(event EventBeginPlay)

(event Collision|EventActorBeginOverlap
  (params (OtherActor :type Actor%20Object%20Reference)))

(event EventTick
  (params (DeltaSeconds :type Float%20%28single-precision%29))
  (Utilities|FlowControl|Sequence
    (:then_0
      (Utilities|FlowControl|DoOnce false :!label _label
        (:Completed
          (Variables|Default|SetOctoState "NewEnumerator1")
          (Timeline|ShootCooldown PlayFromStart
            (:Finished
              (Variables|Default|SetOctoState "NewEnumerator0"))))))
    (:then_1
      (switch Utilities|FlowControl|Switch|SwitchonOctoState (Variables|Default|GetOctoState)
        (:NewEnumerator0
          (CallFunction|Shoot)
          (goto _label Reset))))))

(fn ConstructionScript)